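; BP_ClosingDoor is a one-shot door that swings shut when the first-person player enters its CloseDoorCol trigger.
; The overlap starts looping or playing door audio and a timeline that lerps the static mesh yaw from open to closed.
; When the timeline finishes, the audio stops, a closed sound plays, and the whole actor destroys itself after a short delay.
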(event OnComponentBeginOverlap(CloseDoorCol)
  (params (OverlappedComponent :type Primitive%20Component%20Object%20Reference) (OtherActor :type Actor%20Object%20Reference) (OtherComp :type Primitive%20Component%20Object%20Reference) (OtherBodyIndex :type Integer) (bFromSweep :type Boolean) (SweepResult :type Hit%20Result%20Structure%20%28by%20ref%29))
  (bind _staticmesh (Variables|Default|GetStaticMesh))
  (bind _relativerotation (Variables|/Script/Engine.SceneComponent|GetRelativeRotation _staticmesh))
  (Utilities|Casting|CastToBP_FirstPersonCharacter OtherActor)
  (Audio|Components|Audio|Play (Variables|Default|GetAudio) 0.0)
  (bind _closedoor (Timeline|Timeline PlayFromStart)
    (:Update
      (Transformation|SetRelativeRotation _staticmesh (Math|Rotator|MakeRotator (.roll _relativerotation) (.pitch _relativerotation) (Math|Float|Lerp 124.0 0.0 _closedoor)) false false))
    (:Finished
      (Audio|Components|Audio|StopDelayed (Variables|Default|GetAudio) 0.25)
      (Audio|PlaySound2D "/Game/0_Asset/SFX/Effect/Door/closed.closed" 1.0 1.0 0.0 0 0)
      (Utilities|FlowControl|Delay 1.0)
      (Actor|DestroyActor))))

(event EventBeginPlay)

(event Collision|EventActorBeginOverlap
  (params (OtherActor :type Actor%20Object%20Reference)))

(event EventTick
  (params (DeltaSeconds :type Float%20%28single-precision%29)))

(fn ConstructionScript)