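; One-shot trigger volume that updates the HUD objective when the player arrives without a specific key.
; On box overlap by BP_FirstPersonCharacter, it searches the character's Keys for its KeyIndex.
; If the key is found it destroys itself silently; otherwise it sends ObjectiveTxt to the character's HUD and expires shortly after via lifespan.
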(event OnComponentBeginOverlap(ObjBoxCol)
  (params (OverlappedComponent :type Primitive%20Component%20Object%20Reference) (OtherActor :type Actor%20Object%20Reference) (OtherComp :type Primitive%20Component%20Object%20Reference) (OtherBodyIndex :type Integer) (bFromSweep :type Boolean) (SweepResult :type Hit%20Result%20Structure%20%28by%20ref%29))
  (bind _keyindex (Variables|Default|GetKeyIndex))
  (bind _asbp_first_person_character (Utilities|Casting|CastToBP_FirstPersonCharacter OtherActor))
  (bind _array_element (Utilities|Array|ForEachLoopwithBreak (Variables|/Game/Own/Player/BP_FirstPersonCharacter.BP_FirstPersonCharacter_C|GetKeys _asbp_first_person_character) :!label _label)
    (:LoopBody
      (if (== _array_element _keyindex)
        (Variables|Default|SetGoodKeyFound _array_element)
        (goto _label Break)))
    (:Completed
      (if (== (Variables|Default|GetGoodKeyFound) _keyindex)
        (Actor|DestroyActor)
        (else
          (Default|SetObjective (Variables|/Game/Own/Player/BP_FirstPersonCharacter.BP_FirstPersonCharacter_C|GetHudRef _asbp_first_person_character) (Variables|Default|GetObjective%20Txt))
          (Actor|SetLifeSpan 0.5))))))

(event EventBeginPlay)

(fn ConstructionScript)