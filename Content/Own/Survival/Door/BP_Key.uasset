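; Pickup key actor that the first-person character collects, adding its Index to the character's Keys.
; Overlapping PickUpKeyArea enables input, opens a gate and shows help text on the HUD; leaving reverses all three.
; Interact passes only through the open gate, then stores the key, plays a sound, sets the HUD key image and destroys the actor.
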(event OnComponentBeginOverlap(PickUpKeyArea)
  (params (OverlappedComponent :type Primitive%20Component%20Object%20Reference) (OtherActor :type Actor%20Object%20Reference) (OtherComp :type Primitive%20Component%20Object%20Reference) (OtherBodyIndex :type Integer) (bFromSweep :type Boolean) (SweepResult :type Hit%20Result%20Structure%20%28by%20ref%29))
  (bind _asbp_first_person_character (Utilities|Casting|CastToBP_FirstPersonCharacter OtherActor))
  (Utilities|FlowControl|Sequence
    (:then_0
      (Input|EnableInput (Game|GetPlayerController 0))
      (Utilities|FlowControl|Gate true) ; enters at Open
    )
    (:then_1
      (Default|SetHelpText (Variables|/Game/Own/Player/BP_FirstPersonCharacter.BP_FirstPersonCharacter_C|GetHudRef _asbp_first_person_character) (Variables|Default|GetHelper%20Key%20Txt)))))

(event OnComponentEndOverlap(PickUpKeyArea)
  (params (OverlappedComponent :type Primitive%20Component%20Object%20Reference) (OtherActor :type Actor%20Object%20Reference) (OtherComp :type Primitive%20Component%20Object%20Reference) (OtherBodyIndex :type Integer))
  (bind _asbp_first_person_character (Utilities|Casting|CastToBP_FirstPersonCharacter OtherActor))
  (Utilities|FlowControl|Sequence
    (:then_0
      (Input|DisableInput (Game|GetPlayerController 0))
      (Utilities|FlowControl|Gate true) ; enters at Close
    )
    (:then_1
      (Default|SetHelpText (Variables|/Game/Own/Player/BP_FirstPersonCharacter.BP_FirstPersonCharacter_C|GetHudRef _asbp_first_person_character)))))

(event EventInteract
  (Utilities|FlowControl|Gate true
    (:Exit
      (Utilities|Array|Add (Variables|/Game/Own/Player/BP_FirstPersonCharacter.BP_FirstPersonCharacter_C|GetKeys (stale OnComponentBeginOverlap(PickUpKeyArea) _asbp_first_person_character)) (Variables|Default|GetIndex))
      (Audio|PlaySoundatLocation (Variables|Default|GetPickUpKeySound) (Transformation|GetActorLocation) "0, 0, 0" 1.0 1.0 0.0 0 0 0 0)
      (bind _asbp_first_person_character (Utilities|Casting|CastToBP_FirstPersonCharacter (Game|Player|GetPlayerPawn 0)))
      (Default|SetKeyImage (Variables|/Game/Own/Player/BP_FirstPersonCharacter.BP_FirstPersonCharacter_C|GetHudRef _asbp_first_person_character) (Variables|Default|GetKey%20Image))
      (Actor|DestroyActor))))

(fn ConstructionScript)