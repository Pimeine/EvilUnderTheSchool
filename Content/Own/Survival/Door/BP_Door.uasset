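; Interactable survival-game door that opens once, optionally requiring a matching key from the player's key list.
; An overlap area enables interact input and a gate while the player is inside.
; Opening snaps the mesh's yaw by an angle; both opening and failed key attempts play a sound and report an "Important" AI noise event.
; A monster entering the area has its HasSeenPlayer blackboard flag cleared.
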(event OnComponentBeginOverlap(OpeningArea)
  (params (OverlappedComponent :type Primitive%20Component%20Object%20Reference) (OtherActor :type Actor%20Object%20Reference) (OtherComp :type Primitive%20Component%20Object%20Reference) (OtherBodyIndex :type Integer) (bFromSweep :type Boolean) (SweepResult :type Hit%20Result%20Structure%20%28by%20ref%29))
  (bind _returnvalue (Transformation|GetActorLocation))
  (bind _staticmesh (Variables|Default|GetStaticMesh))
  (bind _asbp_first_person_character (Utilities|Casting|CastToBP_FirstPersonCharacter OtherActor)
    (:then
      (Input|EnableInput (Game|GetPlayerController 0))
      (Utilities|FlowControl|Gate true) ; enters at Open
    )
    (:CastFailed
      (bind _asbp_monster (Utilities|Casting|CastToBP_Monster OtherActor))
      (AI|Components|Blackboard|SetValueasBool (AI|GetBlackboard _asbp_monster) (Utilities|Name|MakeLiteralName "HasSeenPlayer") false))))

(event OnComponentEndOverlap(OpeningArea)
  (params (OverlappedComponent :type Primitive%20Component%20Object%20Reference) (OtherActor :type Actor%20Object%20Reference) (OtherComp :type Primitive%20Component%20Object%20Reference) (OtherBodyIndex :type Integer))
  (bind _returnvalue (Transformation|GetActorLocation))
  (bind _staticmesh (Variables|Default|GetStaticMesh))
  (Utilities|Casting|CastToBP_FirstPersonCharacter OtherActor)
  (Input|DisableInput (Game|GetPlayerController 0))
  (Utilities|FlowControl|Gate true) ; enters at Close
)

(event Input|EnhancedActionEvents|EnhancedInputActionIA_Interact
  (params (ActionValue :type Boolean) (ElapsedSeconds :type Float%20%28double-precision%29) (TriggeredSeconds :type Float%20%28double-precision%29) (InputAction :type Input%20Action%20Object%20Reference :default "/Game/FirstPerson/Input/Actions/IA_Interact.IA_Interact"))
  (bind _returnvalue (Game|GetPlayerController 0))
  (bind _returnvalue_2 (Transformation|GetActorLocation))
  (bind _staticmesh (Variables|Default|GetStaticMesh))
  (bind _returnvalue_3 (Transformation|GetActorLocation _returnvalue))
  (:Triggered
    (if (Variables|Default|GetDoesOpenWithKey)
      (bind _array_element (Utilities|Array|ForEachLoopwithBreak (Variables|/Game/Own/Player/BP_FirstPersonCharacter.BP_FirstPersonCharacter_C|GetKeys (stale OnComponentBeginOverlap(OpeningArea) _asbp_first_person_character)))
        (:LoopBody
          (if (== _array_element (Variables|Default|GetKeyIndex))
            (Variables|Default|SethasRightKey true)))
        (:Completed
          (if (Variables|Default|GethasRightKey)
            (Utilities|FlowControl|Gate true :!label _label
              (:Exit
                (if (not (Variables|Default|GetisDoorOpen))
                  (Variables|Default|SetisDoorOpen true)
                  (Audio|PlaySoundatLocation (Variables|Default|GetOpenDoorSound) _returnvalue_2 "0, 0, 0" 1.0 1.0 0.0 0 0 0 0)
                  (Class|AISenseHearing|ReportNoiseEvent _returnvalue_2 5.0 self 0.0 "Important")
                  (Transformation|SetRelativeRotation _staticmesh (Math|Rotator|MakeRotator 0.0 0.0 (+ (Variables|Default|GetOpenAngle) (.yaw (Transformation|GetWorldRotation _staticmesh)))) false false))))
            (else
              (Audio|PlaySoundatLocation (Variables|Default|GetCloseDoorSound) _returnvalue_3 "0, 0, 0" 1.0 1.0 0.0 0 0 0 0)
              (Class|AISenseHearing|ReportNoiseEvent _returnvalue_3 5.0 self 0.0 "Important")))))
      (else
        (goto _label)))))

(fn ConstructionScript)