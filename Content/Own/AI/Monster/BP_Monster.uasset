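; Monster AI character that senses and chases the player or "Important"-tagged noises and attacks the player in melee.
; Perception updates write noise position, seen flag and chase target to the Blackboard, ignoring safe players as targets, with DoOnce and Gate nodes toggling chase state.
; Every Tick runs a forward sphere trace that, after a delay, turns to an unsafe player, plays the attack montage and deals damage using monster-info struct values.
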(event OnTargetPerceptionUpdated(AIPerception)
  (params (Actor :type Actor%20Object%20Reference) (Stimulus :type AI%20Stimulus%20Structure))
  (bind (_age _expirationage _strength _stimuluslocation _receiverlocation _tag _bsuccessfullysensed) (Utilities|Struct|BreakAIStimulus Stimulus))
  (bind _returnvalue (AI|GetBlackboard 0))
  (bind _returnvalue_2 (AI|GetBlackboard 0))
  (Development|PrintString "Sensed")
  (AI|Components|Blackboard|SetValueasVector (AI|GetBlackboard 0) (Utilities|Name|MakeLiteralName "NoisePosition") _stimuluslocation)
  (bind _asbp_first_person_character (Utilities|Casting|CastToBP_FirstPersonCharacter Actor)
    (:then
      (Development|PrintString "CAST" true true "(R=0.930350,G=1.000000,B=0.000000,A=1.000000)")
      (if (and _bsuccessfullysensed (not (Variables|/Game/Own/Player/BP_FirstPersonCharacter.BP_FirstPersonCharacter_C|GetisSafe _asbp_first_person_character)))
        (Utilities|FlowControl|Sequence
          (:then_0
            (Utilities|FlowControl|DoOnce false :!label _label
              (:Completed
                (AI|Components|Blackboard|SetValueasBool _returnvalue_2 (Utilities|Name|MakeLiteralName "HasSeenPlayer") true)
                (AI|Components|Blackboard|SetValueasObject _returnvalue_2 (Utilities|Name|MakeLiteralName "ToChase") _asbp_first_person_character)
                (Utilities|FlowControl|Gate true :!label _label_2 ; enters at Close
                  (:Exit
                    _)))))
          (:then_1
            (goto _label_3 Reset)))
        (else
          (Utilities|FlowControl|Sequence
            (:then_0
              (goto _label Reset))
            (:then_1
              (Utilities|FlowControl|DoOnce false :!label _label_3
                (:Completed
                  (AI|Components|Blackboard|SetValueasBool (AI|GetBlackboard 0) (Utilities|Name|MakeLiteralName "HasSeenPlayer") false)
                  (goto _label_2 Open)))))))
      (AI|Components|Blackboard|SetValueasObject (AI|GetBlackboard 0) (Utilities|Name|MakeLiteralName "ToChase") 0))
    (:CastFailed
      (Development|PrintString "CAST FAILED" true true "(R=1.000000,G=0.028928,B=0.000000,A=1.000000)")
      (if (== _tag "Important")
        (Development|PrintString "true")
        (Utilities|FlowControl|Sequence
          (:then_0
            (Utilities|FlowControl|DoOnce false :!label _label_4
              (:Completed
                (AI|Components|Blackboard|SetValueasBool _returnvalue (Utilities|Name|MakeLiteralName "HasSeenPlayer") true)
                (AI|Components|Blackboard|SetValueasObject _returnvalue (Utilities|Name|MakeLiteralName "ToChase") Actor)
                (Utilities|FlowControl|Gate true) ; enters at Close
              )))
          (:then_1
            (goto _label_5 Reset)))
        (else
          (Utilities|FlowControl|Sequence
            (:then_0
              (goto _label_4 Reset))
            (:then_1
              (Utilities|FlowControl|DoOnce false :!label _label_5
                (:Completed
                  (AI|Components|Blackboard|SetValueasBool (AI|GetBlackboard 0) (Utilities|Name|MakeLiteralName "HasSeenPlayer") false)
                  (Utilities|FlowControl|Gate true) ; enters at Open
                )))))))))

(event Custom|Attack%20Player
  (bind _returnvalue (Transformation|GetActorLocation))
  (bind _struct_monsterinfo (Variables|Default|GetStruct_MonsterInfo))
  (bind (_outhit _returnvalue_2) (Collision|SphereTraceForObjects _returnvalue (+ _returnvalue (* (Math|Vector|GetForwardVector (Transformation|GetActorRotation)) (.attackingdistance _struct_monsterinfo))) 1.2e+02 (Utilities|Array|MakeArray "ObjectTypeQuery3") false 0 "None"))
  (if _returnvalue_2
    (bind _asbp_first_person_character (Utilities|Casting|CastToBP_FirstPersonCharacter (.HitActor (Collision|BreakHitResult _outhit))))
    (if (not (Variables|/Game/Own/Player/BP_FirstPersonCharacter.BP_FirstPersonCharacter_C|GetisSafe _asbp_first_person_character))
      (Utilities|FlowControl|Delay (.delaybetweenattacks _struct_monsterinfo))
      (Transformation|SetActorRotation (Math|Rotator|FindLookatRotation (Transformation|GetActorLocation) (Transformation|GetActorLocation _asbp_first_person_character)))
      (Animation|PlayAnimMontage "/Game/Own/AI/Monster/Animations/AM_Attack.AM_Attack" 1.0 "None")
      (Default|TakeDamage _asbp_first_person_character (.force (Variables|Default|GetStruct_MonsterInfo))))))

(event EventBeginPlay)

(event Collision|EventActorBeginOverlap
  (params (OtherActor :type Actor%20Object%20Reference)))

(event EventTick
  (params (DeltaSeconds :type Float%20%28single-precision%29))
  (CallFunction|AttackPlayer)
  (Utilities|FlowControl|Gate true
    (:Exit
      (AI|Components|Blackboard|SetValueasObject (AI|GetBlackboard 0) (Utilities|Name|MakeLiteralName "ToChase") 0))))

(fn ConstructionScript)