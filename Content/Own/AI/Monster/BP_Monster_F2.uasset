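; BP_Monster_F2 is a monster AI Blueprint variant that plays its hunt sound as soon as it enters play.
; BeginPlay calls the parent implementation, then assigns HuntSound to the Audio component and starts playback from the beginning.
; It adds no other logic, as Tick and overlap events are disabled placeholders and construction only calls the parent.
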(event EventBeginPlay
  (bind _audio (Variables|Default|GetAudio))
  (|CallParentFunction)
  (Audio|Components|Audio|SetSound _audio (Variables|Default|GetHuntSound))
  (Audio|Components|Audio|Play _audio 0.0))

(event Collision|EventActorBeginOverlap
  (params (OtherActor :type Actor%20Object%20Reference))
  (|CallParentFunction OtherActor) ; This node is disabled and will not be called.\nDrag off pins to build functionality.
)

(event EventTick
  (params (DeltaSeconds :type Float%20%28single-precision%29))
  (|CallParentFunction DeltaSeconds) ; This node is disabled and will not be called.\nDrag off pins to build functionality.
)

(fn ConstructionScript
  (|CallParentFunction))